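; BP_Personaje is a player character Blueprint handling movement, mouse look, jump and crouch input.
; Axis inputs drive movement along actor forward and right vectors and controller yaw and inverted pitch.
; Jump stores CanJump in a flag, jumps, then sets JumpZVelocity to the same value whether moving or stationary.
; Crouch input only toggles a pressed flag, with no crouch call here.
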(event EventBeginPlay)

(event Collision|EventActorBeginOverlap
  (params (OtherActor :type Actor%20Object%20Reference)))

(event EventTick
  (params (DeltaSeconds :type Float%20%28single-precision%29)))

(event Input|AxisEvents|InputAxisMoverArriba
  (params (AxisValue :type Float%20%28single-precision%29))
  ;[1 1 1] Movimiento Personaje
  (Pawn|Input|AddMovementInput (Transformation|GetActorForwardVector) AxisValue false))

(event Input|AxisEvents|InputAxisMoverDerecha
  (params (AxisValue :type Float%20%28single-precision%29))
  ;[1 1 1] Movimiento Personaje
  (Pawn|Input|AddMovementInput (Transformation|GetActorRightVector) AxisValue false))

(event Input|AxisEvents|InputAxisMouseX
  (params (AxisValue :type Float%20%28single-precision%29))
  ;[1 1 1] Mira del Mouse
  (Pawn|Input|AddControllerYawInput AxisValue))

(event Input|AxisEvents|InputAxisMouseY
  (params (AxisValue :type Float%20%28single-precision%29))
  ;[1 1 1] Mira del Mouse
  (Pawn|Input|AddControllerPitchInput (* AxisValue -1.0)))

(event Input|ActionEvents|InputActionSaltar
  (params (Key :type Key%20Structure))
  ;[1 1 1] Saltar
  (:Pressed
    (Variables|Default|SetBotón%20Saltar%20presionado (Character|CanJump))
    (Character|Jump)
    (bind _ascharacter_movement_component (Utilities|Casting|CastToCharacterMovementComponent (Pawn|GetMovementComponent)))
    (if (> (Math|Vector|VectorLength (Variables|/Script/Engine.MovementComponent|GetVelocity _ascharacter_movement_component)) 0.0)
      (Variables|/Script/Engine.CharacterMovementComponent|SetJumpZVelocity _ascharacter_movement_component 4e+02)
      (else
        (Variables|/Script/Engine.CharacterMovementComponent|SetJumpZVelocity _ascharacter_movement_component 4e+02))))
  (:Released
    (Variables|Default|SetBotón%20Saltar%20presionado false)
    (Character|StopJumping)))

(event Input|ActionEvents|InputActionAgacharse
  (params (Key :type Key%20Structure))
  ;[1 1 1] Agacharse
  (:Pressed
    (Variables|Default|SetBotón%20agacharse%20presionado true))
  (:Released
    (Variables|Default|SetBotón%20agacharse%20presionado false)))

(fn ConstructionScript)